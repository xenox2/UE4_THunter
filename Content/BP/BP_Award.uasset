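; BP_Award is the player character, handling world-axis movement, death and lives.
; On start it attaches the audio listener to its headlight and turns its lights red in the "End" level if the game isn't cleared.
; Damage or falling below a height limit triggers a one-time ragdoll death with a voice.
; Death then spends a GameInstance life and expires the actor, or opens "End" when none remain.
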(event Custom|falling
  (bind _returnvalue (Game|GetGameInstance))
  (bind _mesh (Variables|Character|GetMesh))
  (bind _asaward_game_instance (Utilities|Casting|CastToAwardGameInstance _returnvalue))
  (Utilities|FlowControl|DoOnce false
    (:Completed
      (Audio|PlaySound2D "/Game/Audio/death_voice.death_voice" 1.0 1.0 0.0 0 0)
      (Utilities|FlowControl|Sequence
        (:then_0
          (Pawn|Components|CharacterMovement|DisableMovement (Variables|Character|GetCharacterMovement))
          (Collision|SetCollisionProfileName _mesh "Ragdoll" true :!class /Script/Engine.PrimitiveComponent)
          (Physics|SetSimulatePhysics _mesh true))
        (:then_1
          (if (> (Variables|/Game/BP/AwardGameInstance.AwardGameInstance_C|GetLife _asaward_game_instance) 0)
            (Variables|/Game/BP/AwardGameInstance.AwardGameInstance_C|SetLife _asaward_game_instance (- (Variables|/Game/BP/AwardGameInstance.AwardGameInstance_C|GetLife _asaward_game_instance) 1))
            (Actor|SetLifeSpan 3.0)
            (else
              (Utilities|FlowControl|Delay 3.0)
              (Game|OpenLevel(byName) "End"))))))))

(event EventBeginPlay
  (bind _asbp_award_player_controller (Utilities|Casting|CastToBP_AwardPlayerController (Pawn|GetController))
    (:then
      (Class|PlayerController|SetAudioListenerOverride _asbp_award_player_controller (Variables|Default|GetHeadLight) "0, 0, 0" "0, 0, 0"))
    (:CastFailed
      _))
  (bind _returnvalue (Game|GetCurrentLevelName true))
  (if (and (Utilities|Enum|Equal(Enum) _returnvalue "End") (not (Variables|/Game/BP/AwardGameInstance.AwardGameInstance_C|GetisClear (.AsAward%20Game%20Instance (Utilities|Casting|CastToAwardGameInstance (Game|GetGameInstance))))))
    (Rendering|Components|Light|SetLightColor (Variables|Default|GetHeadLight) "(R=1.000000,G=0.000000,B=0.000000,A=1.000000)" true)))

(event Collision|EventActorBeginOverlap
  (params (OtherActor :type Actor%20Object%20Reference)))

(event EventTick
  (params (DeltaSeconds :type Float%20%28single-precision%29))
  (if (<= (Math|Float|Truncate (.z (Transformation|GetActorLocation))) -200)
    (CallFunction|Falling)))

(event Game|Damage|EventAnyDamage
  (params (Damage :type Float%20%28single-precision%29) (DamageType :type Damage%20Type%20Object%20Reference) (InstigatedBy :type Controller%20Object%20Reference) (DamageCauser :type Actor%20Object%20Reference))
  (bind _returnvalue (Game|GetGameInstance))
  (bind _mesh (Variables|Character|GetMesh))
  (bind _asaward_game_instance (Utilities|Casting|CastToAwardGameInstance _returnvalue))
  (Utilities|FlowControl|DoOnce false
    (:Completed
      (Audio|PlaySound2D "/Game/Audio/death_voice.death_voice" 1.0 1.0 0.0 0 0)
      (Utilities|FlowControl|Sequence
        (:then_0
          (Pawn|Components|CharacterMovement|DisableMovement (Variables|Character|GetCharacterMovement))
          (Collision|SetCollisionProfileName _mesh "Ragdoll" true :!class /Script/Engine.PrimitiveComponent)
          (Physics|SetSimulatePhysics _mesh true))
        (:then_1
          (if (> (Variables|/Game/BP/AwardGameInstance.AwardGameInstance_C|GetLife _asaward_game_instance) 0)
            (Variables|/Game/BP/AwardGameInstance.AwardGameInstance_C|SetLife _asaward_game_instance (- (Variables|/Game/BP/AwardGameInstance.AwardGameInstance_C|GetLife _asaward_game_instance) 1))
            (Actor|SetLifeSpan 3.0)
            (else
              (Utilities|FlowControl|Delay 3.0)
              (Game|OpenLevel(byName) "End"))))))))

(event Input|AxisEvents|InputAxisMoveForward
  (params (AxisValue :type Float%20%28single-precision%29))
  (Pawn|Input|AddMovementInput "1.000000, 0, 0" AxisValue false))

(event Input|AxisEvents|InputAxisMoveRight
  (params (AxisValue :type Float%20%28single-precision%29))
  (Pawn|Input|AddMovementInput "0,1.000000, 0" AxisValue false))

(fn ConstructionScript)